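; Barracks defence Blueprint that swings its door open when play begins.
; BeginPlay calls MHandler, which triggers DoorOpen, where the DoorTimer timeline drives the door's yaw; DoorClose reverses it.
; The looping timer for Handler and the staggered spawns at the Arrow's relative location before closing the door are disconnected and never run.
; Handler would call the empty mCall event, then reopen the door.
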(event Custom|mCall)

(event Custom|DoorOpen
  (bind _timer (Timeline|DoorTimer Play)
    (:Update
      (Transformation|SetRelativeRotation (Variables|Default|GetDoor) (Math|Rotator|MakeRotator 0.0 0.0 (* _timer -1e+02)) false false))))

(event Custom|DoorClose
  (bind _timer (Timeline|DoorTimer Reverse)
    (:Update
      (Transformation|SetRelativeRotation (Variables|Default|GetDoor) (Math|Rotator|MakeRotator 0.0 0.0 (* _timer -1e+02)) false false))))

(event Custom|Handler
  (CallFunction|MCall)
  (CallFunction|DoorOpen))

(event Custom|mHandler
  (CallFunction|DoorOpen))

(event EventBeginPlay
  (CallFunction|MHandler))

(fn ConstructionScript)
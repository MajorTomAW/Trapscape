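; Player building component that previews, cycles and places pieces from a building inventory.
; It spawns the selected piece with a blueprint material, and Tick snaps it to a grid at the owner's BuildSpawn arrow with right-angle yaw steps.
; Submitting a placeable piece restores saved materials and enables collision; cancelling destroys it.
; BuildingMode toggles ticking and switches the player between movement-oriented and controller-yaw rotation.
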(event Custom|ShowBuildingBlueprint
  (bind _returnvalue (Components|GetOwner))
  (bind _buildinginventory (Variables|Default|GetBuildingInventory))
  (Variables|Default|GetActiveBuildingBlueprint
    (:then)
    (:else
      (if (Utilities|Array|IsValidIndex _buildinginventory)
        (bind _returnvalue_2 (Game|SpawnActorfromClass (Utilities|Struct|Breaks_info_building (Utilities|Array|Get(acopy) _buildinginventory (Variables|Default|GetTileInt))) (Math|Transform|MakeTransform (Transformation|GetActorLocation _returnvalue) "0, 0, 0" "1.000000,1.000000,1.000000") "AlwaysSpawn" _returnvalue 0))
        (bind _output_get (Variables|Default|SetActiveBuildingBlueprint _returnvalue_2))
        (for _array_element (Actor|GetComponentsByClass _output_get "/Script/Engine.StaticMeshComponent")
          (Utilities|Array|Add (Variables|Default|GetMaterials) (Rendering|Material|GetMaterial _array_element 0))
          (Rendering|Material|SetMaterial _array_element 0 "/Game/Materials/Models/m_blueprint_body.m_blueprint_body"))
        (CallFunction|BuildingMode true)))))

(event Custom|SubmitBuilding
  (bind _activebuildingblueprint (Variables|Default|GetActiveBuildingBlueprint)
    (:then
      (if (Variables|/Game/Blueprints/BuildingSystem/bp_building_base.bp_building_base_C|GetbCanPlaced _activebuildingblueprint)
        (CallFunction|BuildingMode false)
        (Variables|/Game/Blueprints/BuildingSystem/bp_building_base.bp_building_base_C|SetbSubmitted _activebuildingblueprint true)
        (for (_array_element _array_index) (Actor|GetComponentsByClass _activebuildingblueprint "/Script/Engine.StaticMeshComponent")
          (Collision|SetCollisionEnabled _array_element "QueryAndPhysics")
          (Rendering|Material|SetMaterial _array_element 0 (Utilities|Array|Get(acopy) (Variables|Default|GetMaterials) _array_index)))
        (Utilities|Array|Clear (Variables|Default|GetMaterials))
        (Variables|Default|SetActiveBuildingBlueprint 0)))
    (:else)))

(event Custom|NextTile
  (CallFunction|CancelBuilding)
  (Variables|Default|SetTileInt (Math|Integer|SelectInt 0 (+ (Variables|Default|GetTileInt) 1) (> (+ (Variables|Default|GetTileInt) 1) (- (Utilities|Array|Length (Variables|Default|GetBuildingInventory)) 1))))
  (CallFunction|ShowBuildingBlueprint))

(event Custom|PreviousTile
  (CallFunction|CancelBuilding)
  (Variables|Default|SetTileInt (Math|Integer|SelectInt (- (Utilities|Array|Length (Variables|Default|GetBuildingInventory)) 1) (- (Variables|Default|GetTileInt) 1) (< (- (Variables|Default|GetTileInt) 1) 0)))
  (CallFunction|ShowBuildingBlueprint))

(event Custom|CancelBuilding
  (CallFunction|BuildingMode false)
  (bind _activebuildingblueprint (Variables|Default|GetActiveBuildingBlueprint)
    (:then
      (Actor|DestroyActor _activebuildingblueprint)
      (Variables|Default|SetActiveBuildingBlueprint 0))
    (:else)))

(event EventTick
  (params (DeltaSeconds :type Float%20%28single-precision%29))
  (bind _linetracespawn (Variables|Default|GetLinetraceSpawn))
  (bind _activebuildingblueprint (Variables|Default|GetActiveBuildingBlueprint))
  (bind _returnvalue (Transformation|GetWorldLocation _linetracespawn))
  (bind (_x _y _z) (Math|Vector|BreakVector _returnvalue))
  (Variables|Default|GetActiveBuildingBlueprint
    (:then
      (Transformation|SetActorLocation _activebuildingblueprint (Math|Vector|MakeVector (Math|Float|SnapToGrid(Float) _x 2e+02) (Math|Float|SnapToGrid(Float) _y 2e+02) (Math|Float|SnapToGrid(Float) _z 4e+02)) false false)
      (Transformation|SetActorRotation _activebuildingblueprint (Math|Rotator|MakeRotator 0.0 0.0 (Math|Float|SnapToGrid(Float) (.yaw (Transformation|GetActorRotation (Components|GetOwner))) 9e+01))))
    (:else)))

(event EventBeginPlay
  (bind _returnvalue (Components|GetOwner))
  (bind _returnvalue_2 (Actor|GetComponentsbyTag _returnvalue "/Script/Engine.ArrowComponent" "BuildSpawn"))
  (bind _output (Utilities|Array|Get(acopy) _returnvalue_2))
  (Utilities|IsValid _output
    (:Is%20Valid
      (Variables|Default|SetLinetraceSpawn _output))))

(fn BuildingMode
  (params (bEnabled :type Boolean))
  (Components|Tick|SetComponentTickEnabled bEnabled)
  (bind _asbpplayer_base (Utilities|Casting|CastToBPPlayerBase (Components|GetOwner)))
  (Variables|/Script/Engine.CharacterMovementComponent|SetbOrientRotationToMovement (Variables|/Script/Engine.Character|GetCharacterMovement _asbpplayer_base) (not bEnabled))
  (Variables|/Script/Engine.Pawn|SetbUseControllerRotationYaw _asbpplayer_base bEnabled))
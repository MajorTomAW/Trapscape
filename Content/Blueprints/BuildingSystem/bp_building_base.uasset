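; Base Blueprint for placeable buildings that shows whether a not-yet-submitted placement is valid.
; Overlaps on the Restricted component clear CanPlaced and swap every static mesh material to an error blueprint material.
; Ending an overlap sets CanPlaced again, but restores the normal blueprint material only when no other building still overlaps.
; Both handlers do nothing once Submitted is set.
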(event OnComponentBeginOverlap(Restricted)
  (params (OverlappedComponent :type Primitive%20Component%20Object%20Reference) (OtherActor :type Actor%20Object%20Reference) (OtherComp :type Primitive%20Component%20Object%20Reference) (OtherBodyIndex :type Integer) (bFromSweep :type Boolean) (SweepResult :type Hit%20Result%20Structure%20%28by%20ref%29))
  (if (not (Variables|Default|GetbSubmitted))
    (Variables|Default|SetbCanPlaced false)
    (for _array_element (Actor|GetComponentsByClass "/Script/Engine.StaticMeshComponent")
      (for _index (range 0 (- (Rendering|Material|GetNumMaterials _array_element) 1))
        (Rendering|Material|SetMaterial _array_element _index "/Game/Materials/Models/m_blueprint_body_error.m_blueprint_body_error")))))

(event OnComponentEndOverlap(Restricted)
  (params (OverlappedComponent :type Primitive%20Component%20Object%20Reference) (OtherActor :type Actor%20Object%20Reference) (OtherComp :type Primitive%20Component%20Object%20Reference) (OtherBodyIndex :type Integer))
  (if (not (Variables|Default|GetbSubmitted))
    (Variables|Default|SetbCanPlaced true)
    (if (== (Utilities|Array|Length (Collision|GetOverlappingActors (Variables|Default|GetRestricted) "bp_building_base_C" :!class /Script/Engine.PrimitiveComponent)) 0)
      (for _array_element (Actor|GetComponentsByClass "/Script/Engine.StaticMeshComponent")
        (for _index (range 0 (- (Rendering|Material|GetNumMaterials _array_element) 1))
          (Rendering|Material|SetMaterial _array_element _index "/Game/Materials/Models/m_blueprint_body.m_blueprint_body"))))))

(fn ConstructionScript)
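; Player character for Trapscape that handles jumping, shooting and health display.
; Enhanced Input drives jump, and the health component's update event pushes current and max health to the player controller's health message.
; Left mouse fires a debug-drawn Camera-channel line trace from the actor's location along the control rotation, applying damage to the hit actor and reporting a damage event for AI perception.
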(event OnUpdateHealth(HealthComponent)
  (params (NewHealth :type Float%20%28single-precision%29))
  (Class|IntTrapscapePlayercontroller|UpdateHealth(Message) (Pawn|GetController) NewHealth (Class|ACHealthComponent|GetMaxHealth (Variables|Default|GetHealthComponent))))

(event Input|EnhancedActionEvents|EnhancedInputActionia_jump
  (params (ActionValue :type Boolean) (ElapsedSeconds :type Float%20%28double-precision%29) (TriggeredSeconds :type Float%20%28double-precision%29) (InputAction :type Input%20Action%20Object%20Reference :default "/Game/EnhancedInput/actions/ia_jump.ia_jump"))
  (:Triggered
    (Character|Jump))
  (:Completed
    (Character|StopJumping)))

(event Input|MouseEvents|LeftMouseButton
  (params (Key :type Key%20Structure :default "None"))
  (bind _returnvalue (Transformation|GetActorLocation))
  (bind _self self)
  (:Pressed
    (bind (_outhit _returnvalue_2) (Collision|LineTraceByChannel _returnvalue (+ _returnvalue (* (Math|Vector|GetForwardVector (Pawn|GetControlRotation :!class /Script/Engine.Pawn)) 5e+03)) "TraceTypeQuery2" false 0 "ForDuration"))
    (if _returnvalue_2
      (Utilities|IsValid (.HitActor (Collision|BreakHitResult _outhit))
        (:Is%20Valid
          (Game|Damage|ApplyDamage (.HitActor (Collision|BreakHitResult _outhit)) 1.0 0 _self)
          (Class|AISenseDamage|ReportDamageEvent (.HitActor (Collision|BreakHitResult _outhit)) _self 2.0 "0, 0, 0" "0, 0, 0" "None"))))))

(fn ConstructionScript)
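; Test actor that turns to face a sensed actor tagged "player".
; AI perception updates store the player on successful sensing and clear the reference when sensing fails.
; A fast looping timer, started on sensing and never cleared, snaps the whole actor's rotation toward the stored player with a look-at rotation while that reference is valid.
; PurchaseBuilding and GetPlayerController are empty stubs.
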(event OnTargetPerceptionUpdated(AIPerception)
  (params (Actor :type Actor%20Object%20Reference) (Stimulus :type AI%20Stimulus%20Structure))
  (if (Actor|ActorHasTag Actor "player")
    (if (.bsuccessfullysensed Stimulus)
      (Variables|Default|SetActor Actor)
      (Utilities|Time|SetTimerbyEvent (delegate Custom|Timer) 0.01 true)
      (else
        (Variables|Default|SetActor 0)))))

(event Custom|Timer
  (bind _actor (Variables|Default|GetActor)
    (:then
      (Transformation|SetActorRotation (Math|Rotator|FindLookatRotation (Transformation|GetActorLocation) (Transformation|GetActorLocation _actor))))
    (:else)))

(event EventBeginPlay)

(event Collision|EventActorBeginOverlap
  (params (OtherActor :type Actor%20Object%20Reference)))

(fn ConstructionScript)

(fn PurchaseBuilding
  (params (Cost :type Integer) (Callback :type W%20Shop%20Object%20Reference))
  (return 0))

(fn GetPlayerController
  (return 0))
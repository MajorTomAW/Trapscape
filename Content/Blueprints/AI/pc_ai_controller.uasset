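; AI controller for enemies that runs the enemy behavior tree and feeds it targets through the blackboard.
; On possess, it finds the life support actor in the level and stores it as the LifeSupportTarget key.
; AI Perception updates branch by sense: damage records the AttackingActor, while sight updates the TargetActor.
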(event OnTargetPerceptionUpdated(AIPerception)
  (params (Actor :type Actor%20Object%20Reference) (Stimulus :type AI%20Stimulus%20Structure))
  (bind _success (Utilities|SwitchonSense Stimulus)
    (:AISense%20Damage
      (Variables|Default|SetAttackingActor Actor)
      (AI|Components|Blackboard|SetValueasObject (AI|GetBlackboard 0) (Utilities|Name|MakeLiteralName "AttackingActor") (Variables|Default|GetAttackingActor)))
    (:AISense%20%20Sight
      (Variables|Default|SetTargetActor (select _success Actor 0))
      (AI|Components|Blackboard|SetValueasObject (AI|GetBlackboard 0) (Utilities|Name|MakeLiteralName "TargetActor") (Variables|Default|GetTargetActor)))))

(event EventPossess
  (params (PossessedPawn :type Pawn%20Object%20Reference))
  (bind _returnvalue (Actor|GetActorOfClass "/Game/Blueprints/BuildingSystem/LifeSupport/bp_lifesupport.bp_lifesupport_C"))
  (Variables|Default|SetLifeSupport _returnvalue)
  (AI|RunBehaviorTree "/Game/Blueprints/AI/BehaviorTree/bt_enemy_ai.bt_enemy_ai")
  (AI|Components|Blackboard|SetValueasObject (AI|GetBlackboard 0) (Utilities|Name|MakeLiteralName "LifeSupportTarget") (Variables|Default|GetLifeSupport)))

(fn ConstructionScript)
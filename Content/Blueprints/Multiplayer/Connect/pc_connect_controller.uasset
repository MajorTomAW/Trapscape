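; Player controller for the connect screen that shows the connection UI and triggers lobby creation through the game instance.
; On BeginPlay, only the local controller creates the W_connect_ui widget, shows the cursor and locks input to UI only.
; It then waits three seconds and calls CreateLobbyMessage on the game instance, passing itself.
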(event Custom|CreateLobby
  (Utilities|FlowControl|Delay 3.0)
  (Class|IntGameinstance|CreateLobby(Message) (Game|GetGameInstance) self))

(event EventBeginPlay
  (if (Pawn|IsLocalController)
    (bind _returnvalue (UserInterface|CreateWidget "/Game/Blueprints/UI/Multiplayer/Connect/w_connect_ui.w_connect_ui_C" self))
    (UserInterface|Viewport|AddtoViewport _returnvalue 0)
    (Variables|Default|SetbShowMouseCursor true)
    (Input|SetInputModeUIOnly self 0 "LockAlways" false)
    (CallFunction|CreateLobby)))

(fn ConstructionScript)
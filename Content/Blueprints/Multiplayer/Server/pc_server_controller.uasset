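; Player controller for the multiplayer server setup that puts UI widgets on the owning player's screen.
; CreateUI forwards a widget class to cCreateUI, which creates the widget for this controller and adds it to the viewport.
; It then shows the mouse cursor and switches to UI-only input with the mouse locked to the viewport.
; GetPlayerController simply returns the controller itself.
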(event Custom|cCreateUI
  (params (Widget :type User%20Widget%20Class%20Reference))
  (bind _returnvalue (UserInterface|CreateWidget Widget self))
  (UserInterface|Viewport|AddtoViewport _returnvalue 0)
  (Variables|Default|SetbShowMouseCursor true)
  (Input|SetInputModeUIOnly self 0 "LockAlways" false))

(event EventBeginPlay)

(event EventTick
  (params (DeltaSeconds :type Float%20%28single-precision%29)))

(event EventCreateUI
  (params (Widget :type User%20Widget%20Class%20Reference))
  (CallFunction|CCreateUI Widget))

(fn ConstructionScript)

(fn GetPlayerController
  (return self))